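; BP_mara is a player-controlled character, Mara, that carries a sword and performs a slash ability.
; On BeginPlay it spawns a Weapon_Sword and snaps it to the mesh's WeaponHold socket.
; The Ability1 input stops and disables movement, raises the SlashSword flag, then after a fixed delay clears it and restores walking.
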(event `self.ReceiveBeginPlay`
  (bind _returnvalue (`|SpawnActorFromClass` "/Game/Mara/Blueprints/Weapon_Sword.Weapon_Sword_C" (`SceneComponent.GetSocketTransform` (`self.Mesh`) "WeaponHold" "RTS_World") "Undefined" "OverrideRootScale" null null))
  (`self.K2_AttachToComponent` _returnvalue (`self.Mesh`) "WeaponHold" "SnapToTarget" "SnapToTarget" "SnapToTarget" true))

(event `InputAction|Ability1`
  (params (Key :type "Key Structure"))
  (bind _charactermovement (`self.CharacterMovement`))
  (:`Pressed`
    (`CharacterMovementComponent.DisableMovement` _charactermovement)
    (`MovementComponent.StopMovementImmediately` _charactermovement)
    (set `self.SlashSword` true)
    (`KismetSystemLibrary.Delay` 2.0)
    (set `self.SlashSword` false)
    (`CharacterMovementComponent.SetMovementMode` (`self.CharacterMovement`) "MOVE_Walking" 0)))

(fn `UserConstructionScript`)