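; Player controller for mouse-driven movement that shows the cursor and moves the pawn toward the point under it while an input is held.
; Two input actions set either a faster or slower walk speed and toggle a released flag on press and release.
; Each tick, it either calls SimpleMoveToLocation on the cursor's Visibility trace hit, if beyond a minimum distance, or stops movement immediately when released.
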(event `self.ReceiveTick`
  (params (DeltaSeconds :type "Float (single-precision)"))
  (if (`self.isReleased`)
    (`self.CancelMovement`)
    (else
      (`self.MoveToHitLocation`))))

(event `self.ReceiveBeginPlay`
  (set `self.bShowMouseCursor` true) ; 游戏开始显示鼠标指针
)

(event `InputAction|MoveToPoint`
  (params (Key :type "Key Structure"))
  (:`Pressed`
    (set `CharacterMovementComponent.MaxWalkSpeed` 600.0 (`Character.CharacterMovement` (`GameplayStatics.GetPlayerCharacter` 0)))
    (set `self.isReleased` false))
  (:`Released`
    (set `self.isReleased` true)))

(event `InputAction|LeftMoveToPoint`
  (params (Key :type "Key Structure"))
  (:`Pressed`
    (set `CharacterMovementComponent.MaxWalkSpeed` 200.0 (`Character.CharacterMovement` (`GameplayStatics.GetPlayerCharacter` 0)))
    (set `self.isReleased` false))
  (:`Released`
    (set `self.isReleased` true)))

(fn `CancelMovement`
  (`MovementComponent.StopMovementImmediately` (`Character.CharacterMovement` (`GameplayStatics.GetPlayerCharacter` 0))))

(fn `MoveToHitLocation`
  (bind (_bblockinghit _binitialoverlap _time _distance _location) (`GameplayStatics.BreakHitResult` (`self.GetHitResultUnderCursorByChannel` "TraceTypeQuery1")))
  (if (>= (`KismetMathLibrary.VSize` (- (`self.K2_GetActorLocation` (`self.K2_GetPawn`)) _location)) (`self.MinClickDistance`))
    (`AIBlueprintHelperLibrary.SimpleMoveToLocation` self _location)))

(fn `UserConstructionScript`)